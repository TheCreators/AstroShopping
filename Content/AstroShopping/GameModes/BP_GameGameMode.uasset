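; Game mode for AstroShopping that sets up save data and the store manager when play begins.
; On BeginPlay, HandlePersistance uses the PersistenceSubsystem to load the existing save from disk, or creates a new one if none exists.
; It then spawns BP_StoreManager at the level transform and stores the reference in StoreManager.
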(event EventBeginPlay
  (CallFunction|HandlePersistance)
  (bind _returnvalue (Game|SpawnActorfromClass "/Game/AstroShopping/StoreSystem/BP_StoreManager.BP_StoreManager_C" (Class|Actor|GetLevelTransform) "Undefined" "MultiplyWithRoot" 0 0))
  (Variables|Default|SetStoreManager _returnvalue))

(event EventTick
  (params (DeltaSeconds :type Float%20%28single-precision%29)))

(fn ConstructionScript)

(fn HandlePersistance
  (bind _returnvalue (Subsystems|GetPersistenceSubsystem))
  (bind _returnvalue_2 (Class|PersistenceSubsystem|DoesGameSaveExistonDisk (Subsystems|GetPersistenceSubsystem)))
  (if _returnvalue_2
    (Class|PersistenceSubsystem|LoadGameSavefromDisk _returnvalue false)
    (else
      (Class|PersistenceSubsystem|CreateGameSave _returnvalue))))