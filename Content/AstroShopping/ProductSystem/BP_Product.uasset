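; BP_Product is an interactable product actor in AstroShopping that a character can pick up, showing its name on a widget.
; CanInteract allows pickup only when the character is not already holding a product, and a scene point supplies the interaction hint location.
; Interact assigns the product to the character, updates its client holding state and product HUD, then asks the game mode's product manager to despawn it.
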(event EventBeginPlay
  (CallFunction|SetWidgetName (Variables|Default|GetName)))

(event Collision|EventActorBeginOverlap
  (params (OtherActor :type Actor%20Object%20Reference)))

(event EventTick
  (params (DeltaSeconds :type Float%20%28single-precision%29)))

(event EventInteract
  (params (Instigator :type Actor%20Object%20Reference))
  (bind _self self)
  (bind _asbp_astro_shopping_character (Utilities|Casting|CastToBP_AstroShoppingCharacter Instigator))
  (bind _output_get (Variables|/Game/AstroShopping/Character/BP_AstroShoppingCharacter.BP_AstroShoppingCharacter_C|SetProduct _asbp_astro_shopping_character _self))
  (bind _output_get_2 (Variables|/Game/AstroShopping/Character/BP_AstroShoppingCharacter.BP_AstroShoppingCharacter_C|SetIsHoldingProduct _asbp_astro_shopping_character true))
  (Default|SetIsHoldingonClient _asbp_astro_shopping_character _output_get_2)
  (Default|ChangeProductHudonClient _asbp_astro_shopping_character _self (Variables|/Script/AstroShopping.Product|GetQuantity _output_get))
  (bind _asbp_game_game_mode (Utilities|Casting|CastToBP_GameGameMode (Game|GetGameMode)))
  (Class|ProductManager|DespawnProduct (Class|GameGameMode|GetProductManager _asbp_game_game_mode) self))

(fn ConstructionScript
  (CallFunction|SetWidgetName "Product Name"))

(fn CanInteract
  (params (Instigator :type Actor%20Object%20Reference))
  (bind _asbp_astro_shopping_character (Utilities|Casting|CastToBP_AstroShoppingCharacter Instigator))
  (return (not (Variables|/Game/AstroShopping/Character/BP_AstroShoppingCharacter.BP_AstroShoppingCharacter_C|GetIsHoldingProduct _asbp_astro_shopping_character))))

(fn GetInteractionHintLocation
  (return (Transformation|GetWorldLocation (Variables|Default|GetInteractionHintPoint))))

(fn SetWidgetName
  (params (InString :type String))
  (bind _aswbp_product_name (Utilities|Casting|CastToWBP_ProductName (UserInterface|GetWidget (Variables|Default|GetNameWidget))))
  (Default|SetName _aswbp_product_name (Utilities|Text|ToText(String) InString)))