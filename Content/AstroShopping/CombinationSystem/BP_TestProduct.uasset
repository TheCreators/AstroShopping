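; BP_TestProduct is a test product actor in the AstroShopping combination system that players can interact with to pick up.
; Interact passes the instigator to a server pick-up, which prints the player's name and destroys the actor without storing anything.
; A debug sphere marks the actor on Tick until SetMesh assigns a static mesh and disables ticking.
; It always allows interaction and places the interaction hint at its own location.
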(event Custom|Server_PickUp
  (params (Instigator :type Actor%20Object%20Reference))
  (Development|PrintText (Utilities|Text|FormatText "Product is picked up by player: {player}" (Utilities|GetDisplayName Instigator)) true true "(R=0.000000,G=0.660000,B=1.000000,A=1.000000)" 1e+01)
  (Actor|DestroyActor))

(event EventInteract
  (params (Instigator :type Actor%20Object%20Reference))
  (CallFunction|ServerPickUp Instigator))

(event EventTick
  (params (DeltaSeconds :type Float%20%28single-precision%29))
  (Rendering|Debug|DrawDebugSphere (Transformation|GetActorLocation) 1e+01 12 "(R=1.000000,G=0.526150,B=0.000000,A=1.000000)" 0.0))

(fn ConstructionScript)

(fn SetMesh
  (params (NewMesh :type Static%20Mesh%20Object%20Reference))
  (Actor|Tick|SetActorTickEnabled false)
  (Components|StaticMesh|SetStaticMesh (Variables|Default|GetProductMesh) NewMesh))

(fn CanInteract
  (return true))

(fn GetInteractionHintLocation
  (return (Transformation|GetActorLocation)))