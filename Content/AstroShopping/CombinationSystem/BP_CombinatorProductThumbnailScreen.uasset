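; An interactable screen actor that shows a product thumbnail for the shopping combination system and reports its index when interacted with.
; On begin play it creates a dynamic material on its screen and starts disabled and blank.
; Enable downloads the image from a URL into the material, while Deselect dims a loaded thumbnail.
; A four-state mode drives this, allowing interaction only while Enabled, not when selected, deselected or disabled.
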(event Custom|Enable
  (params (ThumbnailUrl :type String))
  (Variables|Default|SetMode "NewEnumerator1")
  (bind _output_get (Variables|Default|SetThumbnail%20Url ThumbnailUrl))
  (bind _texture (|DownloadImage _output_get)
    (:then
      (Rendering|Material|SetScalarParameterValue (Variables|Default|GetMaterial) "TextureVisibility" 1.0 :!class /Script/Engine.MaterialInstanceDynamic))
    (:OnSuccess
      (Rendering|Material|SetTextureParameterValue (Variables|Default|GetMaterial) "Texture" _texture))))

(event Custom|Disable
  (Variables|Default|SetMode "NewEnumerator0")
  (Variables|Default|SetThumbnail%20Url "")
  (Rendering|Material|SetScalarParameterValue (Variables|Default|GetMaterial) "TextureVisibility" 0.0 :!class /Script/Engine.MaterialInstanceDynamic)
  (Rendering|Material|SetTextureParameterValue (Variables|Default|GetMaterial) "Texture" "/Game/AstroShopping/CombinationSystem/T_Empty.T_Empty"))

(event Custom|Select
  (Variables|Default|SetMode "NewEnumerator2"))

(event Custom|Deselect
  (Variables|Default|SetMode "NewEnumerator3")
  (if (Utilities|Array|IsEmpty (Variables|Default|GetThumbnail%20Url))
    (Rendering|Material|SetScalarParameterValue (Variables|Default|GetMaterial) "TextureVisibility" 0.0 :!class /Script/Engine.MaterialInstanceDynamic)
    (else
      (Rendering|Material|SetScalarParameterValue (Variables|Default|GetMaterial) "TextureVisibility" 0.25 :!class /Script/Engine.MaterialInstanceDynamic))))

(event EventBeginPlay
  (bind _returnvalue (Rendering|Material|CreateDynamicMaterialInstance (Variables|Default|GetScreen) 0 "/Game/AstroShopping/CombinationSystem/M_CombinatorProductScreen.M_CombinatorProductScreen" "None" :!class /Script/Engine.PrimitiveComponent))
  (Variables|Default|SetMaterial _returnvalue)
  (CallFunction|Disable))

(event EventInteract
  (params (Instigator :type Actor%20Object%20Reference))
  (Default|CallOnInteraction (Variables|Default|GetThumbnailIndex)))

(fn ConstructionScript)

(fn CanInteract
  (params (Instigator :type Actor%20Object%20Reference))
  (return (Utilities|Select :Index (Variables|Default|GetMode) :NewEnumerator0 false :NewEnumerator1 true :NewEnumerator2 false :NewEnumerator3 false)))

(fn GetInteractionHintLocation
  (return (Transformation|GetActorLocation)))