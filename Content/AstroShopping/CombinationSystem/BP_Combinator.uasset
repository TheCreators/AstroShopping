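; Interactable machine that combines two slotted products into a new one, showing progress, product name and selectable thumbnails.
; Interact requires both slots filled and sends names and prices to the server, or opens a credentials widget if Genie token or proxy key is missing.
; RepNotifies update the widgets and four child-actor screens.
; Screen choices request product loading on the server and multicast the highlight; reset clears slots, and errors raise notifications.
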(event Custom|Server_OnScreenSelected
  (params (Index :type Integer))
  (CallFunction|MulticastonScreenSelected Index))

(event Custom|Multicast_OnScreenSelected
  (params (Index :type Integer))
  (for (_array_element _array_index) (Variables|Default|GetProductThumbnailScreens)
    (if (== _array_index Index)
      (Default|Select _array_element)
      (else
        (Default|Deselect _array_element)))))

(event EventOnRepProgress
  (bind _progressbarwidgetinstance (Variables|Default|GetProgressBarWidgetInstance))
  (Utilities|IsValid _progressbarwidgetinstance
    (:Is%20Valid
      (Default|SetCurrentProgress _progressbarwidgetinstance (Variables|Default|GetProgress)))))

(event EventOnRepProductName
  (bind _productnamewidgetinstance (Variables|Default|GetProductNameWidgetInstance))
  (Utilities|IsValid _productnamewidgetinstance
    (:Is%20Valid
      (Default|SetText _productnamewidgetinstance (Utilities|Text|ToText(String) (Variables|Default|GetProductName))))))

(event EventOnRepProductThumbnailUrls
  (bind _selectedproductindex (Variables|Default|GetSelectedProductIndex))
  (for (_array_element _array_index) (Variables|Default|GetProductThumbnailUrls)
    (Utilities|IsValid (Utilities|Array|Get(acopy) (Variables|Default|GetProductThumbnailScreens) _array_index)
      (:Is%20Valid
        (if (not (Utilities|Array|IsEmpty _array_element))
          (if (Utilities|Enum|NotEqual(Enum) _array_element (Variables|/Game/AstroShopping/CombinationSystem/BP_CombinatorProductThumbnailScreen.BP_CombinatorProductThumbnailScreen_C|GetThumbnail%20Url (Utilities|Array|Get(acopy) (Variables|Default|GetProductThumbnailScreens) _array_index)))
            (Default|Enable (Utilities|Array|Get(acopy) (Variables|Default|GetProductThumbnailScreens) _array_index) _array_element)
            (if (and (!= _selectedproductindex -1) (!= _selectedproductindex _array_index))
              (Default|Deselect (Utilities|Array|Get(acopy) (Variables|Default|GetProductThumbnailScreens) _array_index))))
          (else
            (Default|Disable (Utilities|Array|Get(acopy) (Variables|Default|GetProductThumbnailScreens) _array_index))))))))

(event EventInteract
  (params (Instigator :type Actor%20Object%20Reference))
  (bind _returnvalue (Game|GetPlayerController 0))
  (bind _interactable_slot_1 (Variables|Default|GetInteractable%20Slot%201))
  (bind _interactable_slot_2 (Variables|Default|GetInteractable%20Slot%202))
  (bind _product (Variables|/Game/AstroShopping/InteractionSystem/BP_InteractableSlot.BP_InteractableSlot_C|GetProduct _interactable_slot_2))
  (bind _product_2 (Variables|/Game/AstroShopping/InteractionSystem/BP_InteractableSlot.BP_InteractableSlot_C|GetProduct _interactable_slot_1))
  (bind _returnvalue_2 (Class|AstroShoppingUserSettings|GetAstroShoppingUserSettings))
  (Utilities|IsValid _returnvalue_2
    (:Is%20Valid
      (bind _returnvalue_3 (Class|AstroShoppingUserSettings|GetGenieRefreshToken _returnvalue_2))
      (bind _returnvalue_4 (Class|AstroShoppingUserSettings|GetProxyApiKey _returnvalue_2))
      (if (or (Utilities|Array|IsEmpty _returnvalue_3) (Utilities|Array|IsEmpty _returnvalue_4))
        (bind _returnvalue_5 (UserInterface|CreateWidget "/Game/AstroShopping/CombinationSystem/Widgets/WBP_Credentials.WBP_Credentials_C"))
        (UserInterface|Viewport|AddtoViewport _returnvalue_5 0)
        (Input|SetInputModeUIOnly _returnvalue _returnvalue_5 "DoNotLock" false)
        (Variables|/Script/Engine.PlayerController|SetbShowMouseCursor _returnvalue true)
        (else
          (Class|Combinator|ServerStartCombination (Variables|/Script/AstroShopping.Product|GetName _product_2) (Variables|/Script/AstroShopping.Product|GetName _product) (Variables|/Script/AstroShopping.Product|GetPrice _product_2) (Variables|/Script/AstroShopping.Product|GetPrice _product)))))))

(event EventBeginPlay
  (Utilities|FlowControl|Sequence
    (:then_0
      (bind _aswpb_combinator_progress_bar (Utilities|Casting|CastToWPB_CombinatorProgressBar (UserInterface|GetWidget (Variables|Default|GetProgressWidget))))
      (bind _output_get (Variables|Default|SetProgressBarWidgetInstance _aswpb_combinator_progress_bar))
      (Default|SetMaxProgress _output_get (Variables|Default|GetMaxProgress)))
    (:then_1
      (bind _aswbp_combinator_product_name (Utilities|Casting|CastToWBP_CombinatorProductName (UserInterface|GetWidget (Variables|Default|GetProductNameWidget))))
      (bind _output_get_2 (Variables|Default|SetProductNameWidgetInstance _aswbp_combinator_product_name))
      (Default|SetText _output_get_2))
    (:then_2
      (for _array_element (Utilities|Array|MakeArray (Variables|Default|GetBP_CombinatorProductThumbnailScreen0) (Variables|Default|GetBP_CombinatorProductThumbnailScreen1) (Variables|Default|GetBP_CombinatorProductThumbnailScreen2) (Variables|Default|GetBP_CombinatorProductThumbnailScreen3))
        (bind _asbp_combinator_product_thumbnail_screen (Utilities|Casting|CastToBP_CombinatorProductThumbnailScreen (Variables|/Script/Engine.ChildActorComponent|GetChildActor _array_element)))
        (Utilities|Array|Add (Variables|Default|GetProductThumbnailScreens) _asbp_combinator_product_thumbnail_screen)
        (EventDispatchers|BindEventtoOnInteraction _asbp_combinator_product_thumbnail_screen (EventDispatchers|CreateEvent :!event RequestLoadProduct))))
    (:then_3
      (CallFunction|CreateNotificationSystem))))

(event EventOnReset
  (for _array_element (Utilities|Array|MakeArray (Variables|Default|GetInteractable%20Slot%201) (Variables|Default|GetInteractable%20Slot%202))
    (Utilities|IsValid _array_element
      (:Is%20Valid
        (Default|RemoveProduct _array_element)))))

(event EventShowError
  (params (ErrorMessage :type String))
  (bind _slatecolor (Utilities|Struct|MakeSlateColor "(R=0.400000,G=0.607843,B=0.709804,A=1.000000)"))
  (CallFunction|NotificationRight true "Combination Falied" ErrorMessage _slatecolor _slatecolor (Utilities|Struct|MakeSlateColor "(R=0.000000,G=0.000000,B=0.000000,A=1.000000)") "NewEnumerator5" 1e+01 15.0))

(fn ConstructionScript
  (Utilities|FlowControl|Sequence
    (:then_0
      (bind _asbp_interactable_slot (Utilities|Casting|CastToBP_InteractableSlot (Variables|/Script/Engine.ChildActorComponent|GetChildActor (Variables|Default|GetProductSlot1))))
      (Variables|Default|SetInteractable%20Slot%201 _asbp_interactable_slot))
    (:then_1
      (bind _asbp_interactable_slot_2 (Utilities|Casting|CastToBP_InteractableSlot (Variables|/Script/Engine.ChildActorComponent|GetChildActor (Variables|Default|GetProductSlot2))))
      (Variables|Default|SetInteractable%20Slot%202 _asbp_interactable_slot_2))))

(fn RequestLoadProduct
  (params (ThumbnailIndex :type Integer))
  (Class|Combinator|ServerRequestLoadProduct ThumbnailIndex)
  (CallFunction|ServeronScreenSelected ThumbnailIndex))

(fn GetProductSpawnPoint
  (return (Transformation|GetWorldTransform (Variables|Default|GetProductSpawnPoint))))

(fn CanInteract
  (params (Instigator :type Actor%20Object%20Reference))
  (return (Math|Boolean|ANDBoolean (Variables|/Game/AstroShopping/InteractionSystem/BP_InteractableSlot.BP_InteractableSlot_C|GetIsOccupied (Variables|Default|GetInteractable%20Slot%201)) (Variables|/Game/AstroShopping/InteractionSystem/BP_InteractableSlot.BP_InteractableSlot_C|GetIsOccupied (Variables|Default|GetInteractable%20Slot%202)) (not (Class|Combinator|IsWorking)))))

(fn GetInteractionHintLocation
  (return (Transformation|GetActorLocation)))