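; BP_Shelf is a furniture actor in AstroShopping that holds products in twelve BP_InteractableSlot child actors and exposes a location for bots to interact with it.
; Query functions loop over the slots to report whether any is occupied or to gather the stocked products.
; TakeProduct returns the first product matching an ID and empties its slot through ClearSlot, which resets the product, occupancy flag and mesh.
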(event EventBeginPlay)

(event Collision|EventActorBeginOverlap
  (params (OtherActor :type Actor%20Object%20Reference)))

(event EventTick
  (params (DeltaSeconds :type Float%20%28single-precision%29)))

(fn ConstructionScript)

(fn ClearSlot
  (params (Slot :type Child%20Actor%20Component%20Object%20Reference))
  (bind _asbp_interactable_slot (Utilities|Casting|CastToBP_InteractableSlot (Variables|/Script/Engine.ChildActorComponent|GetChildActor Slot)))
  (if (Utilities|IsValid (Variables|/Game/AstroShopping/InteractionSystem/BP_InteractableSlot.BP_InteractableSlot_C|GetProduct _asbp_interactable_slot))
    (Variables|/Game/AstroShopping/InteractionSystem/BP_InteractableSlot.BP_InteractableSlot_C|SetProduct _asbp_interactable_slot 0)
    (Variables|/Game/AstroShopping/InteractionSystem/BP_InteractableSlot.BP_InteractableSlot_C|SetIsOccupied _asbp_interactable_slot false)
    (Components|StaticMesh|SetStaticMesh (Variables|/Game/AstroShopping/InteractionSystem/BP_InteractableSlot.BP_InteractableSlot_C|GetItemMesh _asbp_interactable_slot) 0)))

(fn GetAllSlots
  (return (Utilities|Array|MakeArray (Variables|Default|GetProductSlot1) (Variables|Default|GetProductSlot2) (Variables|Default|GetProductSlot3) (Variables|Default|GetProductSlot4) (Variables|Default|GetProductSlot5) (Variables|Default|GetProductSlot6) (Variables|Default|GetProductSlot7) (Variables|Default|GetProductSlot8) (Variables|Default|GetProductSlot9) (Variables|Default|GetProductSlot10) (Variables|Default|GetProductSlot11) (Variables|Default|GetProductSlot12))))

(fn GetInteractionLocation
  (return (Transformation|GetWorldLocation (Variables|Default|GetBotLocation))))

(fn GetProducts
  (bind _slots (CallFunction|GetAllSlots))
  (for _array_element _slots
    (bind _asbp_interactable_slot (Utilities|Casting|CastToBP_InteractableSlot (Variables|/Script/Engine.ChildActorComponent|GetChildActor _array_element)))
    (if (Variables|/Game/AstroShopping/InteractionSystem/BP_InteractableSlot.BP_InteractableSlot_C|GetIsOccupied _asbp_interactable_slot)
      (Utilities|Array|Add (LocalVariables|GetAllProducts) (Variables|/Game/AstroShopping/InteractionSystem/BP_InteractableSlot.BP_InteractableSlot_C|GetProduct _asbp_interactable_slot))))
  (return (LocalVariables|GetAllProducts)))

(fn HasProducts
  (bind _slots (CallFunction|GetAllSlots))
  (for _array_element _slots
    (bind _asbp_interactable_slot (Utilities|Casting|CastToBP_InteractableSlot (Variables|/Script/Engine.ChildActorComponent|GetChildActor _array_element)))
    (LocalVariables|SetAreProductsOnShelf (or (Variables|/Game/AstroShopping/InteractionSystem/BP_InteractableSlot.BP_InteractableSlot_C|GetIsOccupied _asbp_interactable_slot) (LocalVariables|GetAreProductsOnShelf))))
  (return (LocalVariables|GetAreProductsOnShelf)))

(fn TakeProduct
  (params (ProductID :type Guid%20Structure%20%28by%20ref%29))
  (bind _slots (CallFunction|GetAllSlots))
  (for _array_element _slots
    (bind _asbp_interactable_slot (Utilities|Casting|CastToBP_InteractableSlot (Variables|/Script/Engine.ChildActorComponent|GetChildActor _array_element)))
    (if (Variables|/Game/AstroShopping/InteractionSystem/BP_InteractableSlot.BP_InteractableSlot_C|GetIsOccupied _asbp_interactable_slot)
      (if (== (Variables|/Script/AstroShopping.Product|GetID (Variables|/Game/AstroShopping/InteractionSystem/BP_InteractableSlot.BP_InteractableSlot_C|GetProduct _asbp_interactable_slot)) ProductID)
        (LocalVariables|SetTakenProduct (Variables|/Game/AstroShopping/InteractionSystem/BP_InteractableSlot.BP_InteractableSlot_C|GetProduct _asbp_interactable_slot))
        (CallFunction|ClearSlot _array_element)
        (return (LocalVariables|GetTakenProduct))))))