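; Checkout register for the shopping game that takes payment for customers' products and manages their queue.
; Products fill eight child-actor slots; processing each slot removes its product, adds to the total and updates the multicast price display.
; Once the belt is empty during serving, interacting credits the StoreManager's balance and stats, then flags payment complete.
; A boolean array tracks queue spots, with positions offset from the first bot location.
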(event Custom|ProcessSlotInteraction
  (params (Slot :type BP%20Interactable%20Slot%20Object%20Reference))
  (bind _product (Variables|/Game/AstroShopping/InteractionSystem/BP_InteractableSlot.BP_InteractableSlot_C|GetProduct Slot))
  (if (Utilities|IsValid _product)
    (Variables|Default|SetCombinedPrice (+ (Variables|Default|GetCombinedPrice) (Variables|/Script/AstroShopping.Product|GetPrice _product)))
    (Variables|Default|SetProductsSold (+ (Variables|Default|GetProductsSold) 1))
    (Default|RemoveProduct Slot)
    (CallFunction|SetPriceTextMulticast)
    (bind _isoccupied (CallFunction|IsOccupied))
    (if (not _isoccupied)
      (CallFunction|SetTextColorMulticast 0 89))))

(event Custom|SetTextColorMulticast
  (params (B :type Byte) (G :type Byte) (R :type Byte) (A :type Byte))
  (Rendering|Components|TextRender|SetTextRenderColor (Variables|Default|GetSellText) (Math|Color|MakeColor B G R A)))

(event Custom|SetPriceTextMulticast
  (Rendering|Components|TextRender|SetText (Variables|Default|GetSoldPriceText) (Utilities|Text|ToText(Integer) (Variables|Default|GetCombinedPrice))))

(event EventBeginPlay
  (bind _slots (CallFunction|GetAllSlots))
  (for _array_element _slots
    (bind _asbp_interactable_slot (Utilities|Casting|CastToBP_InteractableSlot (Variables|/Script/Engine.ChildActorComponent|GetChildActor _array_element)))
    (Variables|/Game/AstroShopping/InteractionSystem/BP_InteractableSlot.BP_InteractableSlot_C|SetIsRegisterSlot _asbp_interactable_slot true)
    (Variables|/Game/AstroShopping/InteractionSystem/BP_InteractableSlot.BP_InteractableSlot_C|SetRegister _asbp_interactable_slot self)))

(event Collision|EventActorBeginOverlap
  (params (OtherActor :type Actor%20Object%20Reference)))

(event EventTick
  (params (DeltaSeconds :type Float%20%28single-precision%29)))

(event EventInteract
  (params (Instigator :type Actor%20Object%20Reference))
  (bind _asbp_astro_shopping_character (Utilities|Casting|CastToBP_AstroShoppingCharacter Instigator))
  (CallFunction|ChangeStats _asbp_astro_shopping_character)
  (Variables|Default|SetCombinedPrice 0)
  (Variables|Default|SetProductsSold 0)
  (Variables|Default|SetPaymentComplete true)
  (Variables|Default|SetIsServing false)
  (CallFunction|SetTextColorMulticast 0 0 188)
  (Utilities|FlowControl|Delay 5.0)
  (CallFunction|SetPriceTextMulticast))

(event EventOccupyQueueSpot
  (params (Index :type Integer))
  (Utilities|Array|SetArrayElem (Variables|Default|GetQueue) Index true))

(event EventFreeQueueSpot
  (params (Index :type Integer))
  (Utilities|Array|SetArrayElem (Variables|Default|GetQueue) Index false))

(event EventPlaceProduct
  (params (Product :type Product%20Object%20Reference))
  (bind _asbp_product (Utilities|Casting|CastToBP_Product Product)
    (:then
      (bind _slots (CallFunction|GetAllSlots))
      (bind _array_element (Utilities|Array|ForEachLoopwithBreak _slots :!label _label)
        (:LoopBody
          (bind _asbp_interactable_slot (Utilities|Casting|CastToBP_InteractableSlot (Variables|/Script/Engine.ChildActorComponent|GetChildActor _array_element)))
          (if (not (Variables|/Game/AstroShopping/InteractionSystem/BP_InteractableSlot.BP_InteractableSlot_C|GetIsOccupied _asbp_interactable_slot))
            (Variables|/Game/AstroShopping/InteractionSystem/BP_InteractableSlot.BP_InteractableSlot_C|SetIsOccupied _asbp_interactable_slot true)
            (Variables|/Game/AstroShopping/InteractionSystem/BP_InteractableSlot.BP_InteractableSlot_C|SetProduct _asbp_interactable_slot _asbp_product)
            (goto _label Break)))))
    (:CastFailed
      (Development|PrintString "Cast of Prodict Failed"))))

(event EventAllProductsPlaced
  (Variables|Default|SetPaymentComplete false)
  (Variables|Default|SetIsServing true))

(fn ConstructionScript)

(fn CountPrice
  (bind _slots (CallFunction|GetAllSlots))
  (for _array_element _slots
    (bind _asbp_interactable_slot (Utilities|Casting|CastToBP_InteractableSlot (Variables|/Script/Engine.ChildActorComponent|GetChildActor _array_element)))
    (if (Utilities|IsValid (Variables|/Game/AstroShopping/InteractionSystem/BP_InteractableSlot.BP_InteractableSlot_C|GetProduct _asbp_interactable_slot))
      (Variables|Default|SetCombinedPrice (+ (Variables|/Script/AstroShopping.Product|GetPrice (Variables|/Game/AstroShopping/InteractionSystem/BP_InteractableSlot.BP_InteractableSlot_C|GetProduct _asbp_interactable_slot)) (Variables|Default|GetCombinedPrice)))
      (Variables|Default|SetProductsSold (+ (Variables|Default|GetProductsSold) 1))))
  (return (Variables|Default|GetCombinedPrice)))

(fn ClearSlots
  (for _array_element (Utilities|Array|MakeArray (Variables|Default|GetProductSlot1) (Variables|Default|GetProductSlot2) (Variables|Default|GetProductSlot3) (Variables|Default|GetProductSlot4) (Variables|Default|GetProductSlot5) (Variables|Default|GetProductSlot6) (Variables|Default|GetProductSlot7) (Variables|Default|GetProductSlot8))
    (bind _asbp_interactable_slot (Utilities|Casting|CastToBP_InteractableSlot (Variables|/Script/Engine.ChildActorComponent|GetChildActor _array_element)))
    (Utilities|IsValid (Variables|/Game/AstroShopping/InteractionSystem/BP_InteractableSlot.BP_InteractableSlot_C|GetProduct _asbp_interactable_slot)
      (:Is%20Valid
        (Default|RemoveProduct _asbp_interactable_slot)))))

(fn ShowPriceinText
  (Rendering|Components|TextRender|SetText (Variables|Default|GetSoldPriceText) (Utilities|Text|ToText(Integer) (Variables|Default|GetCombinedPrice))))

(fn ChangeStats
  (params (InstigatorCharacter :type BP%20Astro%20Shopping%20Character%20Object%20Reference))
  (bind _asbp_game_game_mode (Utilities|Casting|CastToBP_GameGameMode (Game|GetGameMode)))
  (bind _output_get (Variables|/Game/AstroShopping/StoreSystem/BP_StoreManager.BP_StoreManager_C|SetBalance (Variables|/Game/AstroShopping/GameModes/BP_GameGameMode.BP_GameGameMode_C|GetStoreManager _asbp_game_game_mode) (+ (Variables|/Game/AstroShopping/StoreSystem/BP_StoreManager.BP_StoreManager_C|GetBalance (Variables|/Game/AstroShopping/GameModes/BP_GameGameMode.BP_GameGameMode_C|GetStoreManager _asbp_game_game_mode)) (Variables|Default|GetCombinedPrice))))
  (Variables|/Game/AstroShopping/StoreSystem/BP_StoreManager.BP_StoreManager_C|SetMoneyEarnedAmount (Variables|/Game/AstroShopping/GameModes/BP_GameGameMode.BP_GameGameMode_C|GetStoreManager _asbp_game_game_mode) (+ (Variables|/Game/AstroShopping/StoreSystem/BP_StoreManager.BP_StoreManager_C|GetMoneyEarnedAmount (Variables|/Game/AstroShopping/GameModes/BP_GameGameMode.BP_GameGameMode_C|GetStoreManager _asbp_game_game_mode)) (Variables|Default|GetCombinedPrice)))
  (Variables|/Game/AstroShopping/StoreSystem/BP_StoreManager.BP_StoreManager_C|SetProductsSoldAmount (Variables|/Game/AstroShopping/GameModes/BP_GameGameMode.BP_GameGameMode_C|GetStoreManager _asbp_game_game_mode) (+ (Variables|/Game/AstroShopping/StoreSystem/BP_StoreManager.BP_StoreManager_C|GetProductsSoldAmount (Variables|/Game/AstroShopping/GameModes/BP_GameGameMode.BP_GameGameMode_C|GetStoreManager _asbp_game_game_mode)) (Variables|Default|GetProductsSold)))
  (Variables|/Game/AstroShopping/StoreSystem/BP_StoreManager.BP_StoreManager_C|SetCustomersServedAmount (Variables|/Game/AstroShopping/GameModes/BP_GameGameMode.BP_GameGameMode_C|GetStoreManager _asbp_game_game_mode) (+ (Variables|/Game/AstroShopping/StoreSystem/BP_StoreManager.BP_StoreManager_C|GetCustomersServedAmount (Variables|/Game/AstroShopping/GameModes/BP_GameGameMode.BP_GameGameMode_C|GetStoreManager _asbp_game_game_mode)) 1))
  (Default|ChangeHudonServer InstigatorCharacter _output_get))

(fn IsOccupied
  (for _array_element (Utilities|Array|MakeArray (Variables|Default|GetProductSlot1) (Variables|Default|GetProductSlot2) (Variables|Default|GetProductSlot3) (Variables|Default|GetProductSlot4) (Variables|Default|GetProductSlot5) (Variables|Default|GetProductSlot6) (Variables|Default|GetProductSlot7) (Variables|Default|GetProductSlot8))
    (bind _asbp_interactable_slot (Utilities|Casting|CastToBP_InteractableSlot (Variables|/Script/Engine.ChildActorComponent|GetChildActor _array_element)))
    (bind _output_get (LocalVariables|SetAre%20ProductsOnTheBelt (or (Variables|/Game/AstroShopping/InteractionSystem/BP_InteractableSlot.BP_InteractableSlot_C|GetIsOccupied _asbp_interactable_slot) (LocalVariables|GetAre%20ProductsOnTheBelt)))))
  (return _output_get))

(fn GetAllSlots
  (return (Utilities|Array|MakeArray (Variables|Default|GetProductSlot1) (Variables|Default|GetProductSlot2) (Variables|Default|GetProductSlot3) (Variables|Default|GetProductSlot4) (Variables|Default|GetProductSlot5) (Variables|Default|GetProductSlot6) (Variables|Default|GetProductSlot7) (Variables|Default|GetProductSlot8))))

(fn CanAcceptProduct
  (bind _slots (CallFunction|GetAllSlots))
  (for _array_element _slots
    (bind _asbp_interactable_slot (Utilities|Casting|CastToBP_InteractableSlot (Variables|/Script/Engine.ChildActorComponent|GetChildActor _array_element)))
    (if (not (Variables|/Game/AstroShopping/InteractionSystem/BP_InteractableSlot.BP_InteractableSlot_C|GetIsOccupied _asbp_interactable_slot))
      (return true))))

(fn CanInteract
  (params (Instigator :type Actor%20Object%20Reference))
  (bind _isoccupied (CallFunction|IsOccupied))
  (return (and (not _isoccupied) (Variables|Default|GetIsServing))))

(fn GetInteractionHintLocation
  (return (Transformation|GetWorldLocation (Variables|Default|GetServe%20Plane))))

(fn GetLocationinQueue
  (params (Index :type Integer))
  (return (Math|Transform|TransformLocation (Transformation|GetActorTransform) (+ (Variables|/Script/Engine.SceneComponent|GetRelativeLocation (Variables|Default|GetFisrtBotLocation)) (Math|Vector|MakeVector (* Index -120) 0.0 0.0)))))

(fn GetQueueCurrentSize
  (for (_array_element _array_index) (Variables|Default|GetQueue)
    (if (not _array_element)
      (return _array_index))))

(fn IsPaymentComplete
  (return (Variables|Default|GetPaymentComplete)))

(fn IsQueueFull
  (bind _queue (Variables|Default|GetQueue))
  (return (Utilities|Array|Get(acopy) _queue (- (Utilities|Array|Length _queue) 1))))

(fn IsQueueSpotOccupied
  (params (Index :type Integer))
  (return (Utilities|Array|Get(acopy) (Variables|Default|GetQueue) Index)))