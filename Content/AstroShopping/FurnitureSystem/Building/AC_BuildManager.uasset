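; Character component that handles previewing, placing, rotating and selling furniture from DT_Furniture.
; A looping timer line-traces from the camera, moving a preview mesh through a grid-snap macro and tinting it by whether the hit is ground or carries the item's placement tag.
; Placement spawns the item's Blueprint and charges its cost through the character.
; Selling matches actor tags to table rows, credits the cost and destroys the actor.
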(event Custom|FurniturePreview
  (params (Index :type Integer))
  ;[0.07 0.1498 1] Put Tracing Preview on loop
  (Variables|Default|SetFurnitureIndex Index)
  (if (Variables|Default|GetIsNoPreview)
    (Variables|Default|SetIsNoPreview false)
    (bind _returnvalue (Utilities|Time|SetTimerbyEvent (delegate Custom|Tracing) 0.1 true))
    (Variables|Default|SetTracingTimer _returnvalue)
    (else
      (Utilities|Time|ClearandInvalidateTimerbyHandle (Variables|Default|GetTracingTimer))
      (Variables|Default|SetTracingTimer ""))))

(event Custom|Tracing
  (bind _returnvalue (Game|GetPlayerCameraManager 0))
  (bind _returnvalue_2 (Transformation|GetActorLocation _returnvalue))
  ;[0.07 0.1498 1] Put Tracing Preview on loop
  ;[1 0.09089 0.07697] Trace Characters line of sight and get the hit point
  (bind (_outhit _returnvalue_3) (Collision|LineTraceByChannel _returnvalue_2 (+ _returnvalue_2 (* (Transformation|GetActorForwardVector _returnvalue) 6e+02)) "TraceTypeQuery1" false 0 "ForOneFrame"))
  (if _returnvalue_3
    (if (or (Actor|ActorHasTag (.HitActor (Collision|BreakHitResult _outhit)) "ground") (Components|ComponentHasTag (.HitComponent (Collision|BreakHitResult _outhit)) (.OnPlaceTag (Utilities|Struct|BreakS_FurnitureInfo (Utilities|Array|Get(acopy) (Variables|Default|GetDT_FurnitureList) (Variables|Default|GetFurnitureIndex))))))
      (Variables|Default|SetCanBePlaced true)
      (else
        (Variables|Default|SetCanBePlaced false)))
    ;[0.0925 1 0.3109] Show Mesh Preview of the selected furniture item
    (Utilities|FlowControl|Sequence
      (:then_0
        (Utilities|FlowControl|DoOnce false
          (:Completed
            (bind _returnvalue_4 (Game|AddComponentbyClass (Variables|Default|GetPlayerCharacter) "/Script/Engine.StaticMeshComponent" false (Variables|Default|GetRelative%20Transform)))
            (bind _output_get (Variables|Default|SetPreviewMesh _returnvalue_4))
            (Components|StaticMesh|SetStaticMesh _output_get (.Mesh (Utilities|Struct|BreakS_FurnitureInfo (Utilities|Array|Get(acopy) (Variables|Default|GetDT_FurnitureList) (Variables|Default|GetFurnitureIndex))))))))
      (:then_1
        (bind _output_get_2 (Variables|Default|SetRelative%20Transform (Math|Transform|MakeTransform (Utilities|MStoppedSpawnLocation (.Location (Collision|BreakHitResult _outhit))) (Variables|Default|GetPreviewRotation) "1.000000,1.000000,1.000000")))
        (Transformation|SetWorldTransform (Variables|Default|GetPreviewMesh) _output_get_2 false false)
        (for (_ _array_index) (Rendering|Material|GetMaterials (Variables|Default|GetPreviewMesh))
          (Rendering|Material|SetMaterial (Variables|Default|GetPreviewMesh) _array_index (select (Variables|Default|GetCanBePlaced) "/Game/AstroShopping/FurnitureSystem/Building/M_AllowBuild.M_AllowBuild" "/Game/AstroShopping/FurnitureSystem/Building/M_NotAllowedBuild.M_NotAllowedBuild")))
        (Collision|SetCollisionEnabled (Variables|Default|GetPreviewMesh) "NoCollision")))))

(event Custom|ResetBuildingMode
  ;[0.0925 1 0.3109] Show Mesh Preview of the selected furniture item
  (Utilities|FlowControl|DoOnce false) ; enters at Reset
)

(event Custom|StopBuilding
  ;[0.1372 1 0.5315] Stop the mesh preview
  (Variables|Default|SetIsNoPreview true)
  (bind _previewmesh (Variables|Default|GetPreviewMesh)
    (:then
      (Components|StaticMesh|SetStaticMesh _previewmesh 0)
      (Variables|Default|SetPreviewMesh 0)
      (Utilities|Time|ClearandInvalidateTimerbyHandle (Variables|Default|GetTracingTimer))
      (Variables|Default|SetTracingTimer "")
      (CallFunction|ResetBuildingMode))
    (:else)))

(event Custom|PlaceObject
  (bind _dt_furniturelist (Variables|Default|GetDT_FurnitureList))
  (bind _furnitureindex (Variables|Default|GetFurnitureIndex))
  (bind _output (Utilities|Array|Get(acopy) _dt_furniturelist _furnitureindex))
  ;[0.7526 0.3335 1] Spawn object on traced location
  (if (and (not (Variables|Default|GetIsNoPreview)) (Variables|Default|GetCanBePlaced))
    (CallFunction|SpawnActoronServer _output (Variables|Default|GetRelative%20Transform))
    (CallFunction|StopBuilding)
    (Default|BuyFurnitureonServer (Variables|Default|GetPlayerCharacter) (.Cost (Utilities|Struct|BreakS_FurnitureInfo _output)))))

(event Custom|RotatePreview
  ;[0.544 0.5615 1] Rotate the mesh preview by 45 degrees
  (if (not (Variables|Default|GetIsNoPreview))
    (Variables|Default|SetPreviewRotation (Math|Rotator|CombineRotators (.rotation (Variables|Default|GetRelative%20Transform)) "0.000000,45.000000,0.000000"))))

(event Custom|SpawnActorOnServer
  (params (Furniture :type S%20Furniture%20Info%20Structure) (Transform :type Transform))
  ;[0.7526 0.3335 1] Spawn object on traced location
  (Game|SpawnActorfromClass (.blueprint Furniture) Transform "AdjustIfPossibleButAlwaysSpawn" "MultiplyWithRoot" 0 0))

(event Custom|SellFurniture
  (params (Furniture%20Actor :type Actor%20Object%20Reference))
  (bind _array_element (Utilities|Array|ForEachLoopwithBreak (Variables|Default|GetDT_FurnitureList) :!label _label)
    (:LoopBody
      (if (Actor|ActorHasTag Furniture%20Actor (.FurnitureTypeTag (Utilities|Struct|BreakS_FurnitureInfo _array_element)))
        (Variables|Default|SetFurnitureCost (.Cost (Utilities|Struct|BreakS_FurnitureInfo _array_element)))
        (goto _label Break)))
    (:Completed
      (if (!= (Variables|Default|GetFurnitureCost) 0)
        (Default|SellFurnitureonServer (Variables|Default|GetPlayerCharacter) (Variables|Default|GetFurnitureCost))
        (Variables|Default|SetFurnitureCost 0)
        (CallFunction|DestroyActoronServer Furniture%20Actor)))))

(event Custom|DestroyActorOnServer
  (params (Actor :type Actor%20Object%20Reference))
  (Actor|DestroyActor Actor))

(event EventBeginPlay
  (bind _asbp_astro_shopping_character (Utilities|Casting|CastToBP_AstroShoppingCharacter (Components|GetOwner)))
  (Variables|Default|SetPlayerCharacter _asbp_astro_shopping_character)
  (Variables|Default|SetCamera (Variables|/Script/AstroShopping.AstroShoppingCharacter|GetFirstPersonCameraComponent _asbp_astro_shopping_character))
  (bind _outrownames (DataTable|GetDataTableRowNames "/Game/AstroShopping/FurnitureSystem/Building/DT_Furniture.DT_Furniture"))
  (for _array_element _outrownames
    (bind _returnvalue (Utilities|GetDataTableRow "/Game/AstroShopping/FurnitureSystem/Building/DT_Furniture.DT_Furniture" _array_element)
      (:then
        (Utilities|Array|Add (Variables|Default|GetDT_FurnitureList) _returnvalue)))))