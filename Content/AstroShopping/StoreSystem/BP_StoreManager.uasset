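; BP_StoreManager holds the store's persistent stats: balance, products sold, customers served, money earned and ad conversion rate.
; On BeginPlay it binds to the persistence subsystem's game-loaded delegate and requests a load, copying saved StoreStats into its variables when that delegate fires.
; A SaveData event packs those variables back into the save's StoreStats struct, with no caller in this graph.
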(event Custom|OnGameLoaded_Event
  (params (CurrentGameSave :type Astro%20Shopping%20Save%20Game%20Object%20Reference))
  (Class|Saveable|LoadData CurrentGameSave))

(event EventBeginPlay
  (bind _returnvalue (Subsystems|GetPersistenceSubsystem))
  (EventDispatchers|AssignOnGameLoaded _returnvalue (delegate Custom|OnGameLoaded_Event))
  (Class|PersistenceSubsystem|RequestLoad _returnvalue self))

(event Collision|EventActorBeginOverlap
  (params (OtherActor :type Actor%20Object%20Reference)))

(event EventTick
  (params (DeltaSeconds :type Float%20%28single-precision%29)))

(event EventSaveData
  (params (CurrentGameSave :type Astro%20Shopping%20Save%20Game%20Object%20Reference))
  (Variables|/Script/AstroShopping.AstroShoppingSaveGame|SetStoreStats CurrentGameSave (Utilities|Struct|MakeStoreStatsSaveData (Variables|Default|GetBalance) (Variables|Default|GetProductsSoldAmount) (Variables|Default|GetCustomersServedAmount) (Variables|Default|GetMoneyEarnedAmount) (Variables|Default|GetAdsConversionRate))))

(event EventLoadData
  (params (CurrentGameSave :type Astro%20Shopping%20Save%20Game%20Object%20Reference))
  (bind _storestats (Variables|/Script/AstroShopping.AstroShoppingSaveGame|GetStoreStats CurrentGameSave))
  (Variables|Default|SetBalance (.balance _storestats))
  (Variables|Default|SetProductsSoldAmount (.pruductssoldamount _storestats))
  (Variables|Default|SetCustomersServedAmount (.customersservedamount _storestats))
  (Variables|Default|SetMoneyEarnedAmount (.moneyearned _storestats))
  (Variables|Default|SetAdsConversionRate (.adsconversionvalue _storestats)))

(fn ConstructionScript)