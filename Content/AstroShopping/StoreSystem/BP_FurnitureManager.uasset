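; BP_FurnitureManager holds the store's furniture layout as a map of furniture names to transform arrays and persists it through the save game.
; On BeginPlay it binds to the persistence subsystem's load event and requests a load.
; LoadData restores the map and, if never saved before, seeds a default shelf and register.
; SaveData writes the map and saved-before flag back; the manager spawns no furniture itself.
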(event Custom|OnGameLoaded_Event
  (params (CurrentGameSave :type Astro%20Shopping%20Save%20Game%20Object%20Reference))
  (Class|Saveable|LoadData CurrentGameSave))

(event EventBeginPlay
  (bind _returnvalue (Subsystems|GetPersistenceSubsystem))
  (bind _returnvalue_2 (Class|PersistenceSubsystem|DoesGameSaveExistonDisk _returnvalue))
  (Variables|Default|SetWasSavedBefore _returnvalue_2)
  (EventDispatchers|AssignOnGameLoaded _returnvalue (delegate Custom|OnGameLoaded_Event))
  (Class|PersistenceSubsystem|RequestLoad _returnvalue self))

(event EventSaveData
  (params (CurrentGameSave :type Astro%20Shopping%20Save%20Game%20Object%20Reference))
  (Variables|/Script/AstroShopping.AstroShoppingSaveGame|SetFurnitureData CurrentGameSave (Variables|Default|GetFurnitureMap))
  (Variables|/Script/AstroShopping.AstroShoppingSaveGame|SetWasFurnitureSavedBefore CurrentGameSave (Variables|Default|GetWasSavedBefore)))

(event EventLoadData
  (params (CurrentGameSave :type Astro%20Shopping%20Save%20Game%20Object%20Reference))
  (Variables|Default|SetFurnitureMap (Variables|/Script/AstroShopping.AstroShoppingSaveGame|GetFurnitureData CurrentGameSave))
  (bind _output_get (Variables|Default|SetWasSavedBefore (Variables|/Script/AstroShopping.AstroShoppingSaveGame|GetWasFurnitureSavedBefore CurrentGameSave)))
  (if (not _output_get)
    (Utilities|Map|Add (Variables|Default|GetFurnitureMap) "Shelf" (Utilities|Struct|MakeFurnitureLocationSaveData (Utilities|Array|MakeArray (Math|Transform|MakeTransform "1990.000000,-300.000000,30.000000" "0.000000,180.000000,0.000000"))))
    (Utilities|Map|Add (Variables|Default|GetFurnitureMap) "Register" (Utilities|Struct|MakeFurnitureLocationSaveData (Utilities|Array|MakeArray (Math|Transform|MakeTransform "1770.000000,370.000000,30.000000"))))
    (Variables|Default|SetWasSavedBefore true)))

(fn ConstructionScript)