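; Game instance for AstroShopping that handles multiplayer session creation, invite joining and opening the Lobby as a listen server.
; Creating a session and accepting an invite both start a DestroySession, then create or join immediately without waiting for its result.
; Session results are only printed as debug strings; the Lobby travel is a separate event not triggered by session success in this graph.
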(event Custom|CreateAdvancedSession
  (bind _returnvalue (Game|GetPlayerController 0))
  (|DestroySession _returnvalue
    (:then
      (|AdvancedSession 0 _returnvalue 100 0 false true false true true true false false false true false true
        (:OnSuccess
          (Development|PrintString "Created session" true true "(R=0.000000,G=1.000000,B=0.000000,A=1.000000)" 5.0))
        (:OnFailure
          (Development|PrintString "Failed to create session" true true "(R=1.000000,G=0.000000,B=0.000000,A=1.000000)" 5.0))))
    (:OnSuccess
      (Development|PrintString "Destroyed session" true true "(R=0.000000,G=1.000000,B=0.000000,A=1.000000)" 5.0))
    (:OnFailure
      (Development|PrintString "Failed to destroy session or no session existed" true true "(R=1.000000,G=0.000000,B=0.000000,A=1.000000)" 5.0))))

(event Custom|OpenLevel
  (Game|OpenLevel(byObjectReference) "/Game/AstroShopping/Maps/Lobby.Lobby" true "listen"))

(event EventOnSessionInviteAccepted
  (params (LocalPlayerNum :type Integer) (PersonInvited :type BP%20Unique%20Net%20Id%20Structure) (SessionToJoin :type Blueprint%20Session%20Result%20Structure%20%28by%20ref%29))
  (bind _returnvalue (Game|GetPlayerController 0))
  (|DestroySession _returnvalue
    (:then
      (Development|PrintString "Invite Accepted, joining session")
      (|JoinSession _returnvalue SessionToJoin
        (:OnSuccess
          (Development|PrintString "Joined session" true true "(R=0.000000,G=1.000000,B=0.000000,A=1.000000)"))
        (:OnFailure
          (Development|PrintString "Failed to join session" true true "(R=1.000000,G=0.000000,B=0.000000,A=1.000000)"))))
    (:OnSuccess
      (Development|PrintString "Destroyed session" true true "(R=0.000000,G=1.000000,B=0.000000,A=1.000000)" 5.0))
    (:OnFailure
      (Development|PrintString "Failed to destroy session or no session existed" true true "(R=1.000000,G=0.000000,B=0.000000,A=1.000000)" 5.0))))