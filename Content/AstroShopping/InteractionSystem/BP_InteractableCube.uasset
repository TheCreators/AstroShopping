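; BP_InteractableCube is an interactable cube actor in the AstroShopping interaction system that toggles between two materials when used.
; Interact flips the IsOpen flag, whose OnRep calls UpdateMaterial to swap the cube's material for networked state sync.
; It always allows interaction and places its interaction hint at the actor's location.
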(event Custom|UpdateMaterial
  (bind _cube (Variables|Default|GetCube))
  (if (Variables|Default|GetIsOpen)
    (Rendering|Material|SetMaterial _cube 0 (Variables|Default|GetMaterial2))
    (else
      (Rendering|Material|SetMaterial _cube 0 (Variables|Default|GetMaterial1)))))

(event EventInteract
  (params (Instigator :type Actor%20Object%20Reference))
  (Variables|Default|SetIsOpen (not (Variables|Default|GetIsOpen))))

(fn ConstructionScript)

(fn OnRepIsOpen
  (CallFunction|UpdateMaterial))

(fn CanInteract
  (return true))

(fn GetInteractionHintLocation
  (return (Transformation|GetActorLocation)))