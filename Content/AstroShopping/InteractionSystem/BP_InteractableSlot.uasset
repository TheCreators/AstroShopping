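; Interactable slot actor where the astro shopping character places the product it is holding.
; CanInteract allows use only while the character holds a product and the slot is unoccupied.
; Interact clears the character's holding flag, marks the slot occupied and sets ItemMesh to the product's mesh.
; The interaction hint sits at the actor's location, and nothing in the graphs frees an occupied slot.
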(event EventBeginPlay)

(event Collision|EventActorBeginOverlap
  (params (OtherActor :type Actor%20Object%20Reference)))

(event EventTick
  (params (DeltaSeconds :type Float%20%28single-precision%29)))

(event EventInteract
  (params (Instigator :type Actor%20Object%20Reference))
  (bind _asbp_astro_shopping_character (Utilities|Casting|CastToBP_AstroShoppingCharacter Instigator))
  (if (Variables|/Game/AstroShopping/Character/BP_AstroShoppingCharacter.BP_AstroShoppingCharacter_C|GetIsHoldingProduct _asbp_astro_shopping_character)
    (bind _output_get (Variables|Default|SetProduct (Variables|/Game/AstroShopping/Character/BP_AstroShoppingCharacter.BP_AstroShoppingCharacter_C|GetProduct _asbp_astro_shopping_character)))
    (Variables|/Game/AstroShopping/Character/BP_AstroShoppingCharacter.BP_AstroShoppingCharacter_C|SetIsHoldingProduct _asbp_astro_shopping_character false)
    (Variables|Default|SetIsOccupied true)
    (Components|StaticMesh|SetStaticMesh (Variables|Default|GetItemMesh) (Utilities|ResolveSoftReference (Variables|/Script/AstroShopping.Product|GetProductMesh _output_get)))))

(fn ConstructionScript)

(fn CanInteract
  (params (Instigator :type Actor%20Object%20Reference))
  (bind _asbp_astro_shopping_character (Utilities|Casting|CastToBP_AstroShoppingCharacter Instigator))
  (return (and (Variables|/Game/AstroShopping/Character/BP_AstroShoppingCharacter.BP_AstroShoppingCharacter_C|GetIsHoldingProduct _asbp_astro_shopping_character) (not (Variables|Default|GetIsOccupied)))))

(fn GetInteractionHintLocation
  (return (Transformation|GetActorLocation)))