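; Player character for the multiplayer shop game AstroShopping, handling menus, furniture building, held products and store purchases.
; Inputs toggle escape and build menus, drive the ACBuildManager preview, placement and rotation, and drop held products.
; Server events use the GameMode's StoreManager and ProductManager to change the shared balance and spawn products.
; Balance reaches HUDs by multicast and StoreStats RepNotify; debug keys test spawning, sessions and credentials.
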(event Custom|Debug_Server_SpawnProduct
  ;[1 1 1] Debug
  (bind _asbp_game_game_mode (Utilities|Casting|CastToBP_GameGameMode (Game|GetGameMode)))
  (Class|ProductManager|RequestNewProductSpawn (Class|GameGameMode|GetProductManager _asbp_game_game_mode) (Utilities|Struct|MakeProductDataSaveData "Biggest Double Duck" 123 "https://raw.githubusercontent.com/KhronosGroup/glTF-Sample-Assets/main/Models/ClearCoatCarPaint/glTF-Binary/ClearCoatCarPaint.glb") (Guid|NewGuid) (Transformation|GetActorTransform) 10))

(event Custom|Client_OpenStoreWidget
  (bind _returnvalue (Game|GetPlayerController 0))
  ;[0.5147 0.3223 1] Open Widgets
  (bind _returnvalue_2 (UserInterface|CreateWidget "/Game/AstroShopping/UI/ControlCenterUI/WBP_StoreManagerMenu.WBP_StoreManagerMenu_C"))
  (UserInterface|Viewport|AddtoViewport _returnvalue_2 0)
  (Input|SetInputModeUIOnly _returnvalue _returnvalue_2 "DoNotLock" false)
  (Variables|/Script/Engine.PlayerController|SetbShowMouseCursor _returnvalue true))

(event Custom|ChangeProductHudOnClient
  (params (product :type BP%20Product%20Object%20Reference) (quantity :type Integer))
  ;[1 0.5308 0.3718] HUD
  (bind _asastro_shopping_hud (Utilities|Casting|CastToAstroShoppingHUD (HUD|GetHUD (Game|GetPlayerController 0))))
  (Default|SetProductText (Variables|/Game/Blueprints/AstroShoppingHUD.AstroShoppingHUD_C|GetHUD%20ref _asastro_shopping_hud) (Variables|/Script/AstroShopping.Product|GetName product) quantity (Variables|/Script/AstroShopping.Product|GetPrice product)))

(event Custom|SellFurnitureOnServer
  (params (Cost :type Integer))
  ;[1 0.3384 0.9621] Build Logic
  (CallFunction|SellFurniture Cost))

(event Custom|ChangeProductHudVisibilityOnClient
  ;[1 0.5308 0.3718] HUD
  (bind _asastro_shopping_hud (Utilities|Casting|CastToAstroShoppingHUD (HUD|GetHUD (Game|GetPlayerController 0))))
  (Default|SetProductVisibilityHidden (Variables|/Game/Blueprints/AstroShoppingHUD.AstroShoppingHUD_C|GetHUD%20ref _asastro_shopping_hud)))

(event Custom|SetQuantityOnClient
  (params (Quantity :type Integer) (product :type BP%20Product%20Object%20Reference))
  ;[1 1 1] Setting variables
  (Variables|/Script/AstroShopping.Product|SetQuantity product Quantity))

(event Custom|SetProductOnClient
  (params (product :type BP%20Product%20Object%20Reference) (isHolding :type Boolean))
  ;[1 1 1] Setting variables
  (Variables|Default|SetIsHoldingProduct isHolding)
  (Variables|Default|SetProduct product))

(event Custom|SpawnProductOnServer
  (params (Transform :type Transform) (ID :type Guid%20Structure) (Quantity :type Integer))
  ;[0.3361 0.5359 1] Changing balance
  (bind _asbp_game_game_mode (Utilities|Casting|CastToBP_GameGameMode (Game|GetGameMode)))
  (Class|ProductManager|SpawnProduct (Class|GameGameMode|GetProductManager _asbp_game_game_mode) Transform ID Quantity))

(event Custom|SetIsHoldingOnClient
  (params (IsHolding :type Boolean))
  ;[1 1 1] Setting variables
  (Variables|Default|SetIsHoldingProduct IsHolding))

(event Custom|GetStatsFromServer
  ;[0.5083 1 0.5435] Buy logic
  (bind _asbp_game_game_mode (Utilities|Casting|CastToBP_GameGameMode (Game|GetGameMode)))
  (Variables|/Game/AstroShopping/StoreSystem/BP_StoreManager.BP_StoreManager_C|SetUpdateCounter (Variables|/Game/AstroShopping/GameModes/BP_GameGameMode.BP_GameGameMode_C|GetStoreManager _asbp_game_game_mode) (+ (Variables|/Game/AstroShopping/StoreSystem/BP_StoreManager.BP_StoreManager_C|GetUpdateCounter (Variables|/Game/AstroShopping/GameModes/BP_GameGameMode.BP_GameGameMode_C|GetStoreManager _asbp_game_game_mode)) 1))
  (Variables|Default|SetStoreStats (Variables|/Game/AstroShopping/GameModes/BP_GameGameMode.BP_GameGameMode_C|GetStoreManager _asbp_game_game_mode)))

(event Custom|BuyAdsOnServer
  (params (AdsCost :type Integer))
  ;[0.5083 1 0.5435] Buy logic
  (CallFunction|BuyAds AdsCost))

(event Custom|GetProductManagerFromServer
  ;[0.3361 0.5359 1] Changing balance
  (bind _asbp_game_game_mode (Utilities|Casting|CastToBP_GameGameMode (Game|GetGameMode)))
  (bind _productlist (CallFunction|CreateProductList (Variables|/Script/AstroShopping.ProductManager|GetProductData (Class|GameGameMode|GetProductManager _asbp_game_game_mode))))
  (Variables|Default|SetProductDataList _productlist))

(event Custom|BuyProductOnServer
  (params (Cost :type Integer) (Id :type Guid%20Structure) (Location :type Transform))
  ;[0.5083 1 0.5435] Buy logic
  (CallFunction|BuyProduct Cost Id Location))

(event Custom|ChangeHudOnClientMulticast
  (params (NewBalance :type Integer))
  ;[1 0.5308 0.3718] HUD
  (bind _asastro_shopping_hud (Utilities|Casting|CastToAstroShoppingHUD (HUD|GetHUD (Game|GetPlayerController 0))))
  (Default|SetBalanceText (Variables|/Game/Blueprints/AstroShoppingHUD.AstroShoppingHUD_C|GetHUD%20ref _asastro_shopping_hud) NewBalance))

(event Custom|ChangeHudOnServer
  (params (Balance :type Integer))
  ;[1 0.5308 0.3718] HUD
  (CallFunction|ChangeHudonClientMulticast Balance))

(event Custom|TryToBuyFurniture
  (params (DataRowIndex :type Integer))
  (bind _ac_buildmanager (Variables|Default|GetAC_BuildManager))
  (bind _buildmenuwidget (Variables|Default|GetBuildMenuWidget))
  ;[1 0.3384 0.9621] Build Logic
  (bind _asplayer_controller (Utilities|Casting|CastToPlayerController (Pawn|GetController)))
  (Variables|Default|SetIsBuildMenuOpen false)
  (Default|StopTracing _buildmenuwidget)
  (Widget|RemovefromParent _buildmenuwidget)
  (Variables|/Script/Engine.PlayerController|SetbShowMouseCursor _asplayer_controller false)
  (Input|SetInputModeGameOnly _asplayer_controller false)
  (if (Variables|/Game/AstroShopping/FurnitureSystem/Building/AC_BuildManager.AC_BuildManager_C|GetIsNoPreview _ac_buildmanager)
    (Default|FurniturePreview _ac_buildmanager DataRowIndex)
    (else
      (Default|StopBuilding _ac_buildmanager))))

(event Custom|BuyFurnitureOnServer
  (params (Cost :type Integer))
  ;[1 0.3384 0.9621] Build Logic
  (CallFunction|BuyFurniture Cost))

(event Input|EnhancedActionEvents|EnhancedInputActionIA_OpenEscapeMenu
  (params (ActionValue :type Boolean) (ElapsedSeconds :type Float%20%28double-precision%29) (TriggeredSeconds :type Float%20%28double-precision%29) (InputAction :type Input%20Action%20Object%20Reference :default "/Game/AstroShopping/Input/Actions/IA_OpenEscapeMenu.IA_OpenEscapeMenu"))
  ;[0.5147 0.3223 1] Open Widgets
  (:Started
    (if (not (Variables|Default|GetIsEscapeMenuOpen))
      (CallFunction|OpenEscapeMenu)
      (else
        (Variables|Default|SetIsEscapeMenuOpen false)
        (bind _asplayer_controller (Utilities|Casting|CastToPlayerController (Pawn|GetController)))
        (Widget|RemovefromParent (Variables|Default|GetEscapeMenuWidget))
        (Variables|/Script/Engine.PlayerController|SetbShowMouseCursor _asplayer_controller false)
        (Input|SetInputModeGameOnly _asplayer_controller false)))))

(event Input|EnhancedActionEvents|EnhancedInputActionIA_OpenBuildingMenu
  (params (ActionValue :type Boolean) (ElapsedSeconds :type Float%20%28double-precision%29) (TriggeredSeconds :type Float%20%28double-precision%29) (InputAction :type Input%20Action%20Object%20Reference :default "/Game/AstroShopping/Input/Actions/IA_OpenBuildingMenu.IA_OpenBuildingMenu"))
  (bind _buildmenuwidget (Variables|Default|GetBuildMenuWidget))
  ;[1 0.5514 0.2924] Build inputs
  (if (not (Variables|Default|GetIsBuildMenuOpen))
    (if (Variables|/Game/AstroShopping/FurnitureSystem/Building/AC_BuildManager.AC_BuildManager_C|GetIsNoPreview (Variables|Default|GetAC_BuildManager))
      (CallFunction|OpenBuildMenu)
      (else
        (Default|StopBuilding (Variables|Default|GetAC_BuildManager))
        (CallFunction|OpenBuildMenu)))
    (else
      (Variables|Default|SetIsBuildMenuOpen false)
      (bind _asplayer_controller (Utilities|Casting|CastToPlayerController (Pawn|GetController)))
      (Default|StopTracing _buildmenuwidget)
      (Widget|RemovefromParent _buildmenuwidget)
      (Variables|/Script/Engine.PlayerController|SetbShowMouseCursor _asplayer_controller false)
      (Input|SetInputModeGameOnly _asplayer_controller false))))

(event Input|EnhancedActionEvents|EnhancedInputActionIA_PlaceFurniture
  (params (ActionValue :type Boolean) (ElapsedSeconds :type Float%20%28double-precision%29) (TriggeredSeconds :type Float%20%28double-precision%29) (InputAction :type Input%20Action%20Object%20Reference :default "/Game/AstroShopping/Input/Actions/IA_PlaceFurniture.IA_PlaceFurniture"))
  ;[1 0.5514 0.2924] Build inputs
  (:Started
    (Default|PlaceObject (Variables|Default|GetAC_BuildManager))))

(event Input|EnhancedActionEvents|EnhancedInputActionIA_RotateFurniture
  (params (ActionValue :type Boolean) (ElapsedSeconds :type Float%20%28double-precision%29) (TriggeredSeconds :type Float%20%28double-precision%29) (InputAction :type Input%20Action%20Object%20Reference :default "/Game/AstroShopping/Input/Actions/IA_RotateFurniture.IA_RotateFurniture"))
  ;[1 0.5514 0.2924] Build inputs
  (Default|RotatePreview (Variables|Default|GetAC_BuildManager)))

(event Input|EnhancedActionEvents|EnhancedInputActionIA_DropProduct
  (params (ActionValue :type Boolean) (ElapsedSeconds :type Float%20%28double-precision%29) (TriggeredSeconds :type Float%20%28double-precision%29) (InputAction :type Input%20Action%20Object%20Reference :default "/Game/AstroShopping/Input/Actions/IA_DropProduct.IA_DropProduct"))
  (bind _returnvalue (Transformation|GetActorTransform))
  ;[0.3361 0.5359 1] Changing balance
  (:Started
    (if (Variables|Default|GetIsHoldingProduct)
      (Utilities|IsValid (Variables|Default|GetProduct)
        (:Is%20Valid
          (CallFunction|SpawnProductonServer (Math|Transform|MakeTransform (+ (.location _returnvalue) (* (Transformation|GetActorForwardVector) 4e+01)) (.rotation _returnvalue) (.scale _returnvalue)) (Variables|/Script/AstroShopping.Product|GetProductDataID (Variables|Default|GetProduct)) (Variables|/Script/AstroShopping.Product|GetQuantity (Variables|Default|GetProduct)))
          (Variables|Default|SetProduct 0)
          (Variables|Default|SetIsHoldingProduct false)
          (CallFunction|ChangeProductHudVisibilityonClient))
        (:Is%20Not%20Valid
          (Variables|Default|SetIsHoldingProduct false)
          (CallFunction|ChangeProductHudVisibilityonClient))))))

(event EventBeginPlay
  (bind _aswbp_overhead_widget (Utilities|Casting|CastToWBP_OverheadWidget (UserInterface|GetUserWidgetObject (Variables|Default|GetOverheadWidget))))
  (Class|OverheadWidget|SetDisplayText _aswbp_overhead_widget)
  (Networking|SwitchHasAuthority
    (:Authority
      (CallFunction|GetStatsfromServer))
    (:Remote
      (Utilities|FlowControl|Delay 0.2)
      (CallFunction|GetStatsfromServer))))

(event Collision|EventActorBeginOverlap
  (params (OtherActor :type Actor%20Object%20Reference)))

(event EventTick
  (params (DeltaSeconds :type Float%20%28single-precision%29)))

(event Input|KeyboardEvents|DebugKeyC
  (params (Key :type Key%20Structure :default "None") (ActionValue :type Input%20Action%20Value%20Structure))
  ;[1 1 1] Debug
  (:Pressed
    (bind _asbp_astro_shopping_game_instance (Utilities|Casting|CastToBP_AstroShoppingGameInstance (Game|GetGameInstance))
      (:then
        (Default|CreateAdvancedSession _asbp_astro_shopping_game_instance)
        (Default|OpenLevel _asbp_astro_shopping_game_instance))
      (:CastFailed
        (Development|PrintString "Wrong Game Instance Type" true true "(R=1.000000,G=0.000000,B=0.000000,A=1.000000)" 5.0)))))

(event Input|KeyboardEvents|DebugKeyB
  (params (Key :type Key%20Structure :default "None") (ActionValue :type Input%20Action%20Value%20Structure))
  (bind _returnvalue (Game|GetPlayerController 0))
  ;[1 1 1] Debug
  (:Pressed
    (bind _returnvalue_2 (UserInterface|CreateWidget "/Game/AstroShopping/CombinationSystem/Widgets/WBP_Credentials.WBP_Credentials_C"))
    (UserInterface|Viewport|AddtoViewport _returnvalue_2 0)
    (Input|SetInputModeUIOnly _returnvalue _returnvalue_2 "DoNotLock" false)
    (Variables|/Script/Engine.PlayerController|SetbShowMouseCursor _returnvalue true)))

(event Input|KeyboardEvents|DebugKeyP
  (params (Key :type Key%20Structure :default "None") (ActionValue :type Input%20Action%20Value%20Structure))
  ;[1 1 1] Debug
  (:Pressed
    (CallFunction|DebugServerSpawnProduct)))

(fn ConstructionScript)

(fn BuyAds
  (params (Cost :type Integer))
  (bind _asbp_game_game_mode (Utilities|Casting|CastToBP_GameGameMode (Game|GetGameMode)))
  (if (<= Cost (Variables|/Game/AstroShopping/StoreSystem/BP_StoreManager.BP_StoreManager_C|GetBalance (Variables|/Game/AstroShopping/GameModes/BP_GameGameMode.BP_GameGameMode_C|GetStoreManager _asbp_game_game_mode)))
    (bind _output_get (Variables|/Game/AstroShopping/StoreSystem/BP_StoreManager.BP_StoreManager_C|SetBalance (Variables|/Game/AstroShopping/GameModes/BP_GameGameMode.BP_GameGameMode_C|GetStoreManager _asbp_game_game_mode) (- (Variables|/Game/AstroShopping/StoreSystem/BP_StoreManager.BP_StoreManager_C|GetBalance (Variables|/Game/AstroShopping/GameModes/BP_GameGameMode.BP_GameGameMode_C|GetStoreManager _asbp_game_game_mode)) Cost)))
    (Variables|/Game/AstroShopping/StoreSystem/BP_StoreManager.BP_StoreManager_C|SetAdsConversionRate (Variables|/Game/AstroShopping/GameModes/BP_GameGameMode.BP_GameGameMode_C|GetStoreManager _asbp_game_game_mode) (+ (Variables|/Game/AstroShopping/StoreSystem/BP_StoreManager.BP_StoreManager_C|GetAdsConversionRate (Variables|/Game/AstroShopping/GameModes/BP_GameGameMode.BP_GameGameMode_C|GetStoreManager _asbp_game_game_mode)) 0.2))
    (CallFunction|ChangeHudonServer _output_get)))

(fn CreateProductList
  (params (ProductMap :type Map%20of%20Guid%20Structures%20to%20Structs))
  (bind _keys (Utilities|Map|Keys ProductMap))
  (for _array_element _keys
    (Utilities|Array|Add (LocalVariables|GetProducts) (Utilities|Struct|MakeS_Product _array_element (.name (.Value (Utilities|Map|Find ProductMap _array_element))) (.price (.Value (Utilities|Map|Find ProductMap _array_element))))))
  (return (LocalVariables|GetProducts)))

(fn BuyProduct
  (params (Cost :type Integer) (Id :type Guid%20Structure) (Location :type Transform))
  (bind _asbp_game_game_mode (Utilities|Casting|CastToBP_GameGameMode (Game|GetGameMode)))
  (if (<= Cost (Variables|/Game/AstroShopping/StoreSystem/BP_StoreManager.BP_StoreManager_C|GetBalance (Variables|/Game/AstroShopping/GameModes/BP_GameGameMode.BP_GameGameMode_C|GetStoreManager _asbp_game_game_mode)))
    (bind _output_get (Variables|/Game/AstroShopping/StoreSystem/BP_StoreManager.BP_StoreManager_C|SetBalance (Variables|/Game/AstroShopping/GameModes/BP_GameGameMode.BP_GameGameMode_C|GetStoreManager _asbp_game_game_mode) (- (Variables|/Game/AstroShopping/StoreSystem/BP_StoreManager.BP_StoreManager_C|GetBalance (Variables|/Game/AstroShopping/GameModes/BP_GameGameMode.BP_GameGameMode_C|GetStoreManager _asbp_game_game_mode)) Cost)))
    (CallFunction|ChangeHudonServer _output_get)
    (Class|ProductManager|SpawnProduct (Class|GameGameMode|GetProductManager _asbp_game_game_mode) Location Id 10)))

(fn OnRepStoreStats
  (bind _storestats (Variables|Default|GetStoreStats))
  (if (Utilities|IsValid _storestats)
    (bind _asastro_shopping_hud (Utilities|Casting|CastToAstroShoppingHUD (HUD|GetHUD (Game|GetPlayerController 0))))
    (if (Utilities|IsValid (Variables|/Game/Blueprints/AstroShoppingHUD.AstroShoppingHUD_C|GetHUD%20ref _asastro_shopping_hud))
      (Default|SetBalanceText (Variables|/Game/Blueprints/AstroShoppingHUD.AstroShoppingHUD_C|GetHUD%20ref _asastro_shopping_hud) (Variables|/Game/AstroShopping/StoreSystem/BP_StoreManager.BP_StoreManager_C|GetBalance _storestats)))))

(fn OpenBuildMenu
  (Variables|Default|SetIsBuildMenuOpen true)
  (bind _asplayer_controller (Utilities|Casting|CastToPlayerController (Pawn|GetController)))
  (bind _returnvalue (UserInterface|CreateWidget "/Game/AstroShopping/UI/BuildingUI/WBP_BuildMenu.WBP_BuildMenu_C" _asplayer_controller))
  (bind _output_get (Variables|Default|SetBuildMenuWidget _returnvalue))
  (UserInterface|Viewport|AddtoViewport _output_get 0)
  (Variables|/Script/Engine.PlayerController|SetbShowMouseCursor _asplayer_controller true)
  (Input|SetInputModeGameandUI _asplayer_controller 0 "DoNotLock" true false))

(fn OpenEscapeMenu
  (Variables|Default|SetIsEscapeMenuOpen true)
  (bind _asplayer_controller (Utilities|Casting|CastToPlayerController (Pawn|GetController)))
  (bind _returnvalue (UserInterface|CreateWidget "/Game/AstroShopping/UI/WBP_EscapeMenu.WBP_EscapeMenu_C" _asplayer_controller))
  (bind _output_get (Variables|Default|SetEscapeMenuWidget _returnvalue))
  (UserInterface|Viewport|AddtoViewport _output_get 0)
  (Variables|/Script/Engine.PlayerController|SetbShowMouseCursor _asplayer_controller true)
  (Input|SetInputModeGameandUI _asplayer_controller 0 "DoNotLock" true false))

(fn BuyFurniture
  (params (Cost :type Integer))
  (bind _asbp_game_game_mode (Utilities|Casting|CastToBP_GameGameMode (Game|GetGameMode)))
  (if (<= Cost (Variables|/Game/AstroShopping/StoreSystem/BP_StoreManager.BP_StoreManager_C|GetBalance (Variables|/Game/AstroShopping/GameModes/BP_GameGameMode.BP_GameGameMode_C|GetStoreManager _asbp_game_game_mode)))
    (bind _output_get (Variables|/Game/AstroShopping/StoreSystem/BP_StoreManager.BP_StoreManager_C|SetBalance (Variables|/Game/AstroShopping/GameModes/BP_GameGameMode.BP_GameGameMode_C|GetStoreManager _asbp_game_game_mode) (- (Variables|/Game/AstroShopping/StoreSystem/BP_StoreManager.BP_StoreManager_C|GetBalance (Variables|/Game/AstroShopping/GameModes/BP_GameGameMode.BP_GameGameMode_C|GetStoreManager _asbp_game_game_mode)) Cost)))
    (CallFunction|ChangeHudonServer _output_get)))

(fn SellFurniture
  (params (Cost :type Integer))
  (bind _asbp_game_game_mode (Utilities|Casting|CastToBP_GameGameMode (Game|GetGameMode)))
  (bind _output_get (Variables|/Game/AstroShopping/StoreSystem/BP_StoreManager.BP_StoreManager_C|SetBalance (Variables|/Game/AstroShopping/GameModes/BP_GameGameMode.BP_GameGameMode_C|GetStoreManager _asbp_game_game_mode) (+ Cost (Variables|/Game/AstroShopping/StoreSystem/BP_StoreManager.BP_StoreManager_C|GetBalance (Variables|/Game/AstroShopping/GameModes/BP_GameGameMode.BP_GameGameMode_C|GetStoreManager _asbp_game_game_mode)))))
  (CallFunction|ChangeHudonServer _output_get))

(fn OnRepIsStatsReady)