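; BP_StartButton is an interactable button in the lobby that starts the game.
; Interact plays a timeline that offsets the actor from its starting location, then on forward completion marks it pressed, calls StartGame on the LobbyGameMode and reverses the motion.
; CanInteract requires a valid lobby game mode, no loading players and no completed press, which is only flagged when the forward animation ends.
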(event EventBeginPlay
  (Variables|Default|SetStartLocation (Transformation|GetActorLocation))
  (bind _aslobby_game_mode (Utilities|Casting|CastToLobbyGameMode (Game|GetGameMode)))
  (Variables|Default|SetLobbyGameMode _aslobby_game_mode))

(event Collision|EventActorBeginOverlap
  (params (OtherActor :type Actor%20Object%20Reference)))

(event EventTick
  (params (DeltaSeconds :type Float%20%28single-precision%29)))

(event EventInteract
  (params (Instigator :type Actor%20Object%20Reference))
  (bind (_direction _position) (Timeline|Timeline PlayFromStart)
    (:Update
      (Transformation|SetActorLocation (+ _position (Variables|Default|GetStartLocation)) false false))
    (:Finished
      (switch Utilities|FlowControl|Switch|SwitchonETimelineDirection _direction
        (:Forward
          (Variables|Default|SetbWasPressed true)
          (Class|LobbyGameMode|StartGame (Variables|Default|GetLobbyGameMode))
          (Timeline|Timeline ReverseFromEnd))))))

(fn ConstructionScript)

(fn CanInteract
  (params (Instigator :type Actor%20Object%20Reference))
  (bind _lobbygamemode (Variables|Default|GetLobbyGameMode)
    (:then
      (return (and (not (Class|LobbyGameMode|HasLoadingPlayers _lobbygamemode)) (not (Variables|Default|GetbWasPressed)))))
    (:else
      (return false))))

(fn GetInteractionHintLocation
  (return (Transformation|GetActorLocation)))