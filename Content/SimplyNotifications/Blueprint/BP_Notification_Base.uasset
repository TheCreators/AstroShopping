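; Notification helper that creates, shows and clears on-screen UI notifications for the SimplyNotifications system.
; CreateNotificationSystem adds the WBP_SimplyNotify_Base host widget at high Z-order; NotificationRight appends styled WBP_SNotification entries to its RightUP container and scrolls to the end.
; CreateNotificationUICenter removes existing center popups, then creates and returns a configurable two-button WBP_SNotification_UI_Center.
; Host widgets are found through GetAllWidgetsOfClass, which ClearNotifications also uses to empty RightUP.
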(fn CreateNotificationSystem
  (bind _returnvalue (UserInterface|CreateWidget "/Game/SimplyNotifications/Blueprint/UI/WBP_SimplyNotify_Base.WBP_SimplyNotify_Base_C"))
  (bind _output_get (LocalVariables|SetNotification _returnvalue))
  (UserInterface|Viewport|AddtoViewport _output_get 999))

(fn NotificationRight
  (params (Use%20header? :type Boolean) (Text%20header :type String) (Text%20notification :type String) (Color%20text%20header :type Slate%20Color%20Structure) (Color%20text%20info :type Slate%20Color%20Structure) (Background%20color :type Slate%20Color%20Structure) (Notify%20icon%20style :type E_Notify_style%20Enum :default "NewEnumerator1") (Delay%20sec :type Float%20%28double-precision%29) (Border%20radius :type Float%20%28double-precision%29) (Sound%20notify :type Sound%20Base%20Object%20Reference))
  (bind _foundwidgets (Widget|GetAllWidgetsOfClass 0 "/Game/SimplyNotifications/Blueprint/UI/WBP_SimplyNotify_Base.WBP_SimplyNotify_Base_C" false))
  (for _array_element _foundwidgets
    (bind _returnvalue (UserInterface|CreateWidget "/Game/SimplyNotifications/Blueprint/UI/Notifications/WBP_SNotification.WBP_SNotification_C" 0 Use%20header? Text%20header Text%20notification Color%20text%20header Color%20text%20info Background%20color Notify%20icon%20style Delay%20sec Border%20radius Sound%20notify))
    (Widget|Panel|AddChild (Variables|/Game/SimplyNotifications/Blueprint/UI/WBP_SimplyNotify_Base.WBP_SimplyNotify_Base_C|GetRightUP _array_element) _returnvalue)
    (Class|ScrollBox|ScrolltoEnd (Variables|/Game/SimplyNotifications/Blueprint/UI/WBP_SimplyNotify_Base.WBP_SimplyNotify_Base_C|GetRightUP _array_element))))

(fn CreateNotificationUICenter
  (params (Use%20header%20text? :type Boolean) (Use%20text? :type Boolean) (Text%20header :type String) (Text%20notification :type String) (Color%20text%20header :type Slate%20Color%20Structure) (Color%20text%20info :type Slate%20Color%20Structure) (Background%20color :type Slate%20Color%20Structure) (Border%20radius :type Float%20%28double-precision%29) (Delay%20sec :type Float%20%28double-precision%29) (Notify%20icon%20style :type E_Notify_style%20Enum :default "NewEnumerator1") (Width :type Float%20%28double-precision%29) (Height :type Float%20%28double-precision%29) (Use%20delay? :type Boolean) (Auto%20close? :type Boolean) (Remove%20cursor%20if%20auto%20delay%20close :type Boolean) (Remove%20left%20button :type Boolean) (Remove%20right%20button :type Boolean) (Button%20left%20text :type String) (Button%20right%20text :type String) (Color%20button%20left :type Linear%20Color%20Structure :default "(R=0.000000,G=0.510417,B=0.217104,A=1.000000)") (Color%20button%20right :type Linear%20Color%20Structure :default "(R=0.682292,G=0.052832,B=0.120846,A=1.000000)"))
  (bind _foundwidgets (Widget|GetAllWidgetsOfClass 0 "/Game/SimplyNotifications/Blueprint/UI/Notifications/WBP_SNotification_UI_Center.WBP_SNotification_UI_Center_C" false))
  (for _array_element _foundwidgets
    ;[1 1 1] Remove dublicates
    (Widget|RemovefromParent _array_element))
  (bind _returnvalue (UserInterface|CreateWidget "/Game/SimplyNotifications/Blueprint/UI/Notifications/WBP_SNotification_UI_Center.WBP_SNotification_UI_Center_C" 0 Use%20header%20text? Use%20text? Text%20header Text%20notification Color%20text%20header Color%20text%20info Background%20color Border%20radius Delay%20sec Notify%20icon%20style Width Height Use%20delay? Auto%20close? Remove%20cursor%20if%20auto%20delay%20close Remove%20left%20button Remove%20right%20button Button%20left%20text Button%20right%20text Color%20button%20left Color%20button%20right))
  (bind _output_get (LocalVariables|SetNotify _returnvalue))
  (UserInterface|Viewport|AddtoViewport _output_get 15)
  (return _output_get))

(fn ClearNotifications
  (bind _foundwidgets (Widget|GetAllWidgetsOfClass 0 "/Game/SimplyNotifications/Blueprint/UI/WBP_SimplyNotify_Base.WBP_SimplyNotify_Base_C" false))
  (for _array_element _foundwidgets
    (Widget|Panel|ClearChildren (Variables|/Game/SimplyNotifications/Blueprint/UI/WBP_SimplyNotify_Base.WBP_SimplyNotify_Base_C|GetRightUP _array_element))))